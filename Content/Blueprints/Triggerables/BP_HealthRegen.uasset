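; BP_HealthRegen is a health pickup that restores a random amount of health to an actor with a BP_HealthComp.
; Its Overlapped event calls RegenerateHealth on that component and is consumed only if the call returns true.
; Consumption hides the Cross, disables Trigger collision and attaches a green zap Niagara effect to the consumer.
; After a short delay the pickup reappears and re-enables collision, so it is reusable.
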(event `Consumed`
  (params (`Consumed By` :type "Actor Object Reference"))
  (`SceneComponent.SetVisibility` (`self.Cross`) false true)
  (`PrimitiveComponent.SetCollisionEnabled` (`self.Trigger`) "NoCollision")
  (`NiagaraFunctionLibrary.SpawnSystemAttached` "/Game/Vefects/Zap_VFX/VFX/Zap/Particles/NS_Zap_04_Green.NS_Zap_04_Green" (`Actor.RootComponent` `Consumed By`) "None" (0.0 0.0 0.0) (struct) "SnapToTarget")
  (`KismetSystemLibrary.Delay` 5.0)
  (`SceneComponent.SetVisibility` (`self.Cross`) true true)
  (`PrimitiveComponent.SetCollisionEnabled` (`self.Trigger`) "QueryAndPhysics"))

(event `self.Overlapped`
  (params (OtherActor :type "Actor Object Reference"))
  (bind _returnvalue (`self.GetComponentByClass` OtherActor "/Game/Components/BP_HealthComp.BP_HealthComp_C"))
  (`/Game/EditorBlueprintResources/StandardMacros.IsValid` _returnvalue
    (:`Is Valid`
      (bind _regensuccessful (`/Game/Components/BP_HealthComp.RegenerateHealth` _returnvalue (`KismetMathLibrary.RandomFloatInRange` 10.0 50.0)))
      (if _regensuccessful
        (`self.Consumed` OtherActor)))))

(fn `UserConstructionScript`
  (`parent.UserConstructionScript`))