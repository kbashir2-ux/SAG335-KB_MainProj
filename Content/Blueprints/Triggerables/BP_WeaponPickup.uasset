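; BP_WeaponPickup is a world pickup that offers a weapon class to characters that touch it.
; On overlap with a BP_CharacterBase it passes WeaponClass to that character's WeaponPickupOverlap and destroys itself only if that returns true.
; The construction script sets the static mesh from the Visual default of the weapon class, so one Blueprint can represent any weapon.
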(event `self.Overlapped`
  (params (OtherActor :type "Actor Object Reference"))
  (bind _asbp_character_base (cast `/Game/PlayerAssets/BP_CharacterBase` OtherActor))
  (bind _true (`/Game/PlayerAssets/BP_CharacterBase.WeaponPickupOverlap` _asbp_character_base (`self.WeaponClass`)))
  (if _true
    (`self.K2_DestroyActor`)))

(fn `UserConstructionScript`
  (`parent.UserConstructionScript`)
  (`StaticMeshComponent.SetStaticMesh` (`self.StaticMesh`) (`.Visual` (defaults `Object` (`self.WeaponClass`)))))